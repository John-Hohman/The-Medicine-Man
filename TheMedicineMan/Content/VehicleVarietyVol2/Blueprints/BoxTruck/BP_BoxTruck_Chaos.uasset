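; Player-driven Chaos box truck pawn with throttle, brake, steering, handbrake, toggleable spotlights, horn, and a crash sound on overlapping BP_City.
; Tick maps engine RPM to a rev sound parameter, widens FOV with speed and swings the spring arm with steering.
; Handbrake drives skid, smoke and screech effects, checking whether a wheel is airborne.
; BeginPlay creates the HUD and a mouse-controlled music player; unused boost and drift-angle logic remains unwired.
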(event EventTick
  (params (DeltaSeconds :type Float%20%28single-precision%29))
  (bind _tire_screech_cue (Variables|Default|GetTire_Screech_Cue))
  ;[1 1 1] Revving
  (Audio|Parameter|SetFloatParameter (Variables|Default|GetMSS_richiemcmullen_Rev) "RPM Range" (Math|Float|MapRangeClamped (Class|ChaosWheeledVehicleMovementComponent|GetEngineRotationSpeed (Variables|Default|GetVehicle%20Componenet)) 1.2e+03 5e+03 0.0 1.0) :!class /Script/AudioExtensions.AudioParameterControllerInterface)
  ;[1 1 1] Camera
  (CallFunction|CameraInput)
  ;[1 1 1] Skidding
  (CallFunction|CheckSkidding)
  ;[1 1 1] Tire Screech
  (if (Variables|Default|GetIs%20Handbrake%20on?)
    (for _array_element (Variables|/Script/ChaosVehicles.ChaosWheeledVehicleMovementComponent|GetWheels (Variables|Default|GetVehicle%20Componenet))
      _)
    (if (Class|ChaosVehicleWheel|IsinAir _array_element)
      (Class|AudioComponent|SetPaused _tire_screech_cue true)
      (else
        (Class|AudioComponent|SetPaused _tire_screech_cue false)))))

(event EventBeginPlay
  (bind _aschaos_wheeled_vehicle_movement_component (Utilities|Casting|CastToChaosWheeledVehicleMovementComponent (Variables|Default|GetVehicleMovementComponent)))
  (Variables|Default|SetVehicle%20Componenet _aschaos_wheeled_vehicle_movement_component)
  ;[1 1 1] Radio
  (bind _returnvalue (UserInterface|CreateWidget "/Game/Widgets/UMG_MusicPlayer.UMG_MusicPlayer_C"))
  (UserInterface|Viewport|AddtoViewport _returnvalue 0)
  (Variables|Default|SetMusic%20Player%20UMG _returnvalue)
  (bind _returnvalue_2 (UserInterface|CreateWidget "/Game/Widgets/MenuWidgets/HUD/W_HUD.W_HUD_C"))
  (UserInterface|Viewport|AddtoViewport _returnvalue_2 0)
  ;[1 1 1] Lights
  (Rendering|SetVisibility (Variables|Default|GetSpotLight) false false)
  ;[1 1 1] Horn
  (Utilities|FlowControl|Sequence
    (:then_0
      (Audio|Components|Audio|Stop (Variables|Default|GetHonk_mixdown_Cue)))
    (:then_1
      ;[1 1 1] Tire Screech
      (Class|AudioComponent|SetPaused (Variables|Default|GetTire_Screech_Cue) true))))

(event Collision|EventActorBeginOverlap
  (params (OtherActor :type Actor%20Object%20Reference))
  ;[1 1 1] Crashing
  (Utilities|Casting|CastToBP_City OtherActor)
  (Audio|PlaySound2D "/Game/Sounds/SC_supersouper_carhit.SC_supersouper_carhit" 1.0 1.0 0.0 0 0))

(event Input|ActionEvents|InputActionHandbrake
  (params (Key :type Key%20Structure :default "None"))
  (bind _vehiclemovementcomponent (Variables|Default|GetVehicleMovementComponent))
  (bind _skid2 (Variables|Default|GetSkid2))
  (:Pressed
    (Class|ChaosVehicleMovementComponent|SetHandbrakeInput _vehiclemovementcomponent true)
    (Variables|Default|SetIs%20Handbrake%20on? true)
    ;[1 1 1] Skid Marks
    (if (> (Vehicle|GetForwardSpeed (Variables|Default|GetVehicleMovementComponent)) 5e+02)
      (Components|Activation|Activate _skid2 false)))
  (:Released
    (Class|ChaosVehicleMovementComponent|SetHandbrakeInput _vehiclemovementcomponent false)
    (Variables|Default|SetIs%20Handbrake%20on? false)
    (Components|Activation|Deactivate _skid2)))

(event Input|AxisEvents|InputAxisMoveRight
  (params (AxisValue :type Float%20%28single-precision%29))
  (Class|ChaosVehicleMovementComponent|SetSteeringInput (Variables|Default|GetVehicleMovementComponent) AxisValue)
  (Variables|Default|SetSteering%20Angle AxisValue))

(event Input|AxisEvents|InputAxisMoveForward
  (params (AxisValue :type Float%20%28single-precision%29))
  (Class|ChaosVehicleMovementComponent|SetThrottleInput (Variables|Default|GetVehicleMovementComponent) AxisValue))

(event Input|AxisEvents|InputAxisReverse/Brake
  (params (AxisValue :type Float%20%28single-precision%29))
  (Class|ChaosVehicleMovementComponent|SetBrakeInput (Variables|Default|GetVehicleMovementComponent) AxisValue))

(event Input|MouseEvents|LeftMouseButton
  (params (Key :type Key%20Structure :default "None"))
  (bind _honk_mixdown_cue (Variables|Default|GetHonk_mixdown_Cue))
  ;[1 1 1] Horn
  (:Pressed
    (Audio|Components|Audio|Play _honk_mixdown_cue 0.0))
  (:Released
    (Audio|Components|Audio|Stop _honk_mixdown_cue)))

(event Input|MouseEvents|MouseWheelUp
  (params (Key :type Key%20Structure :default "None"))
  ;[1 1 1] Radio
  (:Pressed
    (Default|NextSong (Variables|Default|GetMusic%20Player%20UMG))))

(event Input|MouseEvents|RightMouseButton
  (params (Key :type Key%20Structure :default "None"))
  ;[1 1 1] Lights
  (:Pressed
    (Utilities|FlowControl|FlipFlop
      (:A
        (Rendering|SetVisibility (Variables|Default|GetSpotLight) true false))
      (:B
        (Rendering|SetVisibility (Variables|Default|GetSpotLight) false false)
        ;[1 1 1] Horn
        (Utilities|FlowControl|Sequence
          (:then_0
            (Audio|Components|Audio|Stop (Variables|Default|GetHonk_mixdown_Cue)))
          (:then_1
            ;[1 1 1] Tire Screech
            (Class|AudioComponent|SetPaused (Variables|Default|GetTire_Screech_Cue) true)))))))

(event Input|MouseEvents|MouseWheelDown
  (params (Key :type Key%20Structure :default "None"))
  ;[1 1 1] Radio
  (:Pressed
    (Default|PreviousSong (Variables|Default|GetMusic%20Player%20UMG))))

(event Input|KeyboardEvents|SpaceBar
  (params (Key :type Key%20Structure :default "None"))
  (bind _tire_screech_cue (Variables|Default|GetTire_Screech_Cue))
  ;[1 1 1] Tire Screech
  (:Pressed
    (if (Variables|Default|GetIs%20Handbrake%20on?)
      (for _array_element (Variables|/Script/ChaosVehicles.ChaosWheeledVehicleMovementComponent|GetWheels (Variables|Default|GetVehicle%20Componenet))
        _)
      (if (Class|ChaosVehicleWheel|IsinAir _array_element)
        (Class|AudioComponent|SetPaused _tire_screech_cue true :!label _label)
        (else
          (Class|AudioComponent|SetPaused _tire_screech_cue false)))))
  (:Released
    (goto _label)))

(event Input|MouseEvents|MiddleMouseButton
  (params (Key :type Key%20Structure :default "None"))
  ;[1 1 1] Radio
  (:Pressed
    (Default|Play/Pause (Variables|Default|GetMusic%20Player%20UMG))))

(fn ConstructionScript)

(fn CameraInput
  (bind _vehiclemovementcomponent (Variables|Default|GetVehicleMovementComponent))
  (bind _springarm (Variables|Default|GetSpringArm))
  (bind _returnvalue (Class|ChaosVehicleMovementComponent|GetForwardSpeedMPH _vehiclemovementcomponent))
  ;[1 1 1] Camera Zoom
  (switch int (Variables|Default|GetCamera%20Index)
    (:Default
      (Camera|SetFieldOfView (Variables|Default|GetCamera) (Math|Float|MapRangeClamped _returnvalue 0.0 1e+02 9e+01 105.0))
      (Transformation|SetRelativeRotation _springarm (Math|Interpolation|RInterpTo (Variables|/Script/Engine.SceneComponent|GetRelativeRotation _springarm) (Math|Rotator|MakeRotator 0.0 -13.0 (Math|Float|Clamp(Float) (* (Variables|Default|GetSteering%20Angle) (Math|Float|MapRangeClamped _returnvalue 1.0 45.0 -4.0 -4.0)) -45.0 45.0)) (Utilities|Time|GetWorldDeltaSeconds) 3.0) false false))))

(fn CheckSkidding
  (Utilities|CheckSkidding 0 (Variables|Default|GetSkid1))
  (Utilities|CheckSkidding 0 (Variables|Default|GetSkid2))
  (Utilities|CheckSkidding 0 (Variables|Default|GetNS_Smoke))
  (Utilities|CheckSkidding 0 (Variables|Default|GetNS_Smoke1))
  (return))