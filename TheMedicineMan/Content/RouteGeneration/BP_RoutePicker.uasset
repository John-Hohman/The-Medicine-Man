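; Route picker that builds random routes from route markers and manages a pedestrian pickup with a destination marker.
; On BeginPlay it fills and reveals a route of unique markers, then starts a looping timer that spawns one pedestrian at a random spawner.
; Random picks retry until valid: destinations avoid the current route, and new routes avoid the last marker and destination.
; UpdatePedestrian flags the pedestrian as gathered and reveals the destination with a pedestrian material.
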(event Custom|NewRoute
  (bind _currroute (Variables|Default|GetCurrRoute))
  ;[1 1 1] Create New Route
  (Variables|Default|SetCurrMarker 0)
  (Utilities|FlowControl|Delay 0.2)
  (for _index (range 0 4)
    (bind _output_get (Variables|Default|SetTest (.OutItem (Utilities|Array|Random (Variables|Default|GetRouteMarkers))) :!label _label))
    (bind _returnvalue (Utilities|Array|AddUnique _currroute _output_get))
    (if (== _returnvalue -1)
      (Utilities|FlowControl|Delay 0.2 :!label _label_2)
      (Development|PrintString (Utilities|String|ToString(Integer) (Variables|/Game/RouteGeneration/BP_RouteMarker.BP_RouteMarker_C|GetRouteValue _output_get)) true true "(R=1.000000,G=0.000000,B=0.055031,A=1.000000)" 1e+01)
      (goto _label)
      (elif (or (== _output_get (Variables|Default|GetLastMarker)) (== _output_get (Variables|Default|GetDestinationMarker)))
        (Utilities|Array|RemoveIndex _currroute (Utilities|Array|LastIndex _currroute))
        (goto _label_2)
        (else
          (Development|PrintString (Utilities|String|ToString(Integer) (Variables|/Game/RouteGeneration/BP_RouteMarker.BP_RouteMarker_C|GetRouteValue _output_get)) true true "(R=0.012786,G=1.000000,B=0.000000,A=1.000000)" 1e+01)))))
  (Utilities|FlowControl|Delay 1.0)
  (for (_array_element _array_index) (Variables|Default|GetCurrRoute)
    (CallFunction|ChangeVisible _array_index)
    (Development|PrintString (Utilities|String|ToString(Integer) (Variables|/Game/RouteGeneration/BP_RouteMarker.BP_RouteMarker_C|GetRouteValue _array_element)) true true "(R=0.976841,G=0.000000,B=1.000000,A=1.000000)" 1e+01)))

(event Custom|SpawnPedestrian
  ;[1 1 1] Spawn Pedestrian
  (if (not (Variables|Default|GetPedestrianSpawned?))
    (Game|SpawnActorfromClass "/Game/RouteGeneration/BP_Pedestrian.BP_Pedestrian_C" (Transformation|GetActorTransform (.OutItem (Utilities|Array|Random (Variables|Default|GetPedestrianSpawners)))) "Undefined" "MultiplyWithRoot" 0 0)
    (bind _output_get (Variables|Default|SetDestinationMarker (.OutItem (Utilities|Array|Random (Variables|Default|GetRouteMarkers))) :!label _label))
    (for _array_element (Variables|Default|GetCurrRoute)
      (if (== _array_element _output_get)
        (Variables|Default|SetDestinationCheck true)))
    (if (Variables|Default|GetDestinationCheck)
      (Variables|Default|SetDestinationCheck false)
      (Utilities|FlowControl|Delay 0.2)
      (goto _label)
      (else
        (Variables|Default|SetDestinationCheck false)
        (Variables|Default|SetPedestrianSpawned? true)))))

(event Custom|ChangeVisible
  (params (Index :type Integer))
  ;[1 1 1] Change Visibility
  (Rendering|SetVisibility (Variables|/Game/RouteGeneration/BP_RouteMarker.BP_RouteMarker_C|GetCube (Utilities|Array|Get(acopy) (Variables|Default|GetCurrRoute) Index)) true false))

(event Custom|Update%20Pedestrian
  (bind _destinationmarker (Variables|Default|GetDestinationMarker))
  (bind _cube (Variables|/Game/RouteGeneration/BP_RouteMarker.BP_RouteMarker_C|GetCube _destinationmarker))
  ;[1 1 1] Change Pedestrian
  (Variables|Default|SetPedestrianGathered? true)
  (Rendering|Material|SetMaterial _cube 0 "/Game/Materials/MI_Pedestrian.MI_Pedestrian")
  (Rendering|SetVisibility _cube true false))

(event EventBeginPlay
  (bind _currroute (Variables|Default|GetCurrRoute))
  ;[1 1 1] Create Starting Route
  (Utilities|FlowControl|Delay 0.2)
  (for _index (range 0 4)
    (bind _returnvalue (Utilities|Array|AddUnique _currroute (.OutItem (Utilities|Array|Random (Variables|Default|GetRouteMarkers))) :!label _label))
    (if (== _returnvalue -1)
      (goto _label)
      (else
        (Development|PrintString (Utilities|String|ToString(Integer) (Variables|/Game/RouteGeneration/BP_RouteMarker.BP_RouteMarker_C|GetRouteValue (Utilities|Array|Get(acopy) _currroute _index))) true true "(R=0.012786,G=1.000000,B=0.000000,A=1.000000)" 1e+01))))
  (Development|PrintString "Hello")
  (for (_ _array_index) (Variables|Default|GetCurrRoute)
    (CallFunction|ChangeVisible _array_index))
  ;[1 1 1] Spawn Pedestrian
  (Utilities|Time|SetTimerbyEvent (delegate Custom|SpawnPedestrian) 11.0 true))

(fn ConstructionScript)