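; BP_Pedestrian is a pickup pedestrian in the route generation system that hands its destination to the route picker.
; When the player pawn overlaps its box, it sets BP_RoutePicker's DestinationMarker to its own Destination, calls UpdatePedestrian and destroys itself.
; A timer started shortly after BeginPlay otherwise removes it after a minute and clears the picker's PedestrianSpawned flag.
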(event OnComponentBeginOverlap(Box)
  (params (OverlappedComponent :type Primitive%20Component%20Object%20Reference) (OtherActor :type Actor%20Object%20Reference) (OtherComp :type Primitive%20Component%20Object%20Reference) (OtherBodyIndex :type Integer) (bFromSweep :type Boolean) (SweepResult :type Hit%20Result%20Structure%20%28by%20ref%29))
  (if (== OtherActor (Game|Player|GetPlayerPawn 0))
    (bind _returnvalue (Actor|GetActorOfClass "/Game/RouteGeneration/BP_RoutePicker.BP_RoutePicker_C"))
    (bind _output_get (Variables|/Game/RouteGeneration/BP_RoutePicker.BP_RoutePicker_C|SetDestinationMarker _returnvalue (Variables|Default|GetDestination)))
    (Development|PrintString (Utilities|String|ToString(Integer) (Variables|/Game/RouteGeneration/BP_RouteMarker.BP_RouteMarker_C|GetRouteValue _output_get)))
    (Default|UpdatePedestrian _returnvalue)
    (Actor|DestroyActor)))

(event Custom|Kill%20actor
  (bind _returnvalue (Actor|GetActorOfClass "/Game/RouteGeneration/BP_RoutePicker.BP_RoutePicker_C"))
  (Variables|/Game/RouteGeneration/BP_RoutePicker.BP_RoutePicker_C|SetPedestrianSpawned? _returnvalue false)
  (Actor|DestroyActor))

(event EventBeginPlay
  (Utilities|FlowControl|Delay 0.5)
  (Development|PrintString (Utilities|String|ToString(Integer) (Variables|Default|GetMarkerSpawned)))
  (Utilities|Time|SetTimerbyEvent (delegate Custom|Kill%20actor) 6e+01))

(fn ConstructionScript)