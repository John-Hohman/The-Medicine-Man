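; BP_RouteMarker is a checkpoint that the player pawn triggers by overlapping its box; its cube starts hidden.
; The current route marker hides itself and advances BP_RoutePicker's index, requesting a new route at the fifth marker or a visibility update otherwise.
; If it is instead the picker's pedestrian destination, it hides, clears its cube material and resets the picker's destination and spawned flag.
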(event OnComponentBeginOverlap(Box)
  (params (OverlappedComponent :type Primitive%20Component%20Object%20Reference) (OtherActor :type Actor%20Object%20Reference) (OtherComp :type Primitive%20Component%20Object%20Reference) (OtherBodyIndex :type Integer) (bFromSweep :type Boolean) (SweepResult :type Hit%20Result%20Structure%20%28by%20ref%29))
  (bind _cube (Variables|Default|GetCube))
  ;[1 1 1] Check Correct Marker
  (if (== OtherActor (Game|Player|GetPlayerPawn 0))
    (bind _returnvalue (Actor|GetActorOfClass "/Game/RouteGeneration/BP_RoutePicker.BP_RoutePicker_C"))
    (Variables|Default|SetPickerRef _returnvalue)
    (if (== self (Utilities|Array|Get(acopy) (Variables|/Game/RouteGeneration/BP_RoutePicker.BP_RoutePicker_C|GetCurrRoute _returnvalue) (Variables|/Game/RouteGeneration/BP_RoutePicker.BP_RoutePicker_C|GetCurrMarker _returnvalue)))
      (bind _output_get (Variables|/Game/RouteGeneration/BP_RoutePicker.BP_RoutePicker_C|SetCurrMarker (Variables|Default|GetPickerRef) (+ (Variables|/Game/RouteGeneration/BP_RoutePicker.BP_RoutePicker_C|GetCurrMarker _returnvalue) 1)))
      (Development|PrintString (Utilities|GetDisplayName _returnvalue) true true "(R=0.000000,G=1.000000,B=0.133730,A=1.000000)" 5.0)
      (Rendering|SetVisibility (Variables|Default|GetCube) false false)
      (if (== _output_get 5)
        (Default|NewRoute (Variables|Default|GetPickerRef))
        (else
          (Default|ChangeVisible (Variables|Default|GetPickerRef))))
      (else
        ;[1 1 1] Check Pedestrian Marker
        (Utilities|IsValid (Variables|/Game/RouteGeneration/BP_RoutePicker.BP_RoutePicker_C|GetDestinationMarker (Variables|Default|GetPickerRef))
          (:Is%20Valid
            (if (== (Variables|/Game/RouteGeneration/BP_RoutePicker.BP_RoutePicker_C|GetDestinationMarker (Variables|Default|GetPickerRef)) self)
              (Development|PrintString (Utilities|GetDisplayName _returnvalue) true true "(R=0.000000,G=1.000000,B=0.133730,A=1.000000)" 5.0)
              (Variables|/Game/RouteGeneration/BP_RoutePicker.BP_RoutePicker_C|SetDestinationMarker (Variables|Default|GetPickerRef) 0)
              (Rendering|SetVisibility _cube false false)
              (Rendering|Material|SetMaterial _cube 0 0)
              (Variables|/Game/RouteGeneration/BP_RoutePicker.BP_RoutePicker_C|SetPedestrianSpawned? (Variables|Default|GetPickerRef) false)
              (else
                (Development|PrintString (Utilities|GetDisplayName _returnvalue) true true "(R=1.000000,G=0.000000,B=0.105670,A=1.000000)" 5.0 :!label _label))))
          (:Is%20Not%20Valid
            (goto _label)))))))

(fn ConstructionScript
  (Rendering|SetVisibility (Variables|Default|GetCube) false false))