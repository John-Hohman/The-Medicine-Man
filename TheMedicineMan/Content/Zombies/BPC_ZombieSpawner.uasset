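; Spawner component that populates the game with zombies around its attach parent's location.
; Each tick, while ZombieCount has not exceeded MaxZombieCount, it spawns a batch of random classes from Zombies, so the total can overshoot the cap.
; Spawns get random yaw, fixed height and randomized offsets, with both axes using the X distance limits.
; ZombieCount only increments here.
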(event Custom|SpawnZombies
  (bind _returnvalue (Transformation|GetAttachParent))
  (bind _maxspawndistancex (Variables|Default|GetMaxSpawnDistanceX))
  (bind _minspawndistancex (Variables|Default|GetMinSpawnDistanceX))
  (bind _maxspawndistancex_2 (Variables|Default|GetMaxSpawnDistanceX))
  (bind _returnvalue_2 (Transformation|GetWorldLocation _returnvalue))
  (bind _returnvalue_3 (* _maxspawndistancex -1.0))
  (bind _returnvalue_4 (Math|Random|RandomFloatinRange _returnvalue_3 _maxspawndistancex))
  (for _index (range 0 10)
    (Game|SpawnActorfromClass (.OutItem (Utilities|Array|Random (Variables|Default|GetZombies))) (Math|Transform|MakeTransform (+ (Math|Vector|MakeVector (.x _returnvalue_2) (.y _returnvalue_2) 0.0) (Math|Vector|MakeVector (+ (Math|Random|RandomFloatinRange _minspawndistancex _maxspawndistancex_2) _returnvalue_4) (+ (Math|Random|RandomFloatinRange _minspawndistancex _maxspawndistancex_2) _returnvalue_4) 9e+01)) (Math|Rotator|MakeRotator 0.0 0.0 (Math|Random|RandomFloatinRange 0.0 359.0)) "1.000000,1.000000,1.000000") "AdjustIfPossibleButAlwaysSpawn" "MultiplyWithRoot" 0 0)
    (Math|Integer|IncrementInt (Variables|Default|GetZombieCount))))

(event EventTick
  (params (DeltaSeconds :type Float%20%28single-precision%29))
  (if (>= (Variables|Default|GetMaxZombieCount) (Variables|Default|GetZombieCount))
    (CallFunction|SpawnZombies)))